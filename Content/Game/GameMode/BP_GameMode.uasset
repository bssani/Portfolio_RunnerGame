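; Game mode for an endless-runner style game that builds the track at BeginPlay and runs a time-based score.
; A startup loop chains random tiles, spawning each at the previous BP_MasterTile's attach transform.
; AddMap counts straight tiles and inserts a random jump tile after every eight.
; Each loop pass also adds a BP_RunningWidget to the viewport and re-sets the looping IncrementScore timer.
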(event `self.ReceiveBeginPlay`
  ;[1 1 1] 레벨 만들기
  ;;[1 1 1] 몇번 반복할것인가
  (for _ (range 21)
    (`self.AddMap`)
    ;[1 1 1] UI and Display
    (bind _returnvalue (`|CreateWidget` "/Game/Game/UI/BP_RunningWidget.BP_RunningWidget_C"))
    (`UserWidget.AddToViewport` _returnvalue 0)
    (bind _returnvalue_2 (`KismetSystemLibrary.K2_SetTimer` null "IncrementScore" 0.6 true))
    (set `self.TimerHandler` _returnvalue_2)))

(fn `AddMap`
  (bind _class (`self.Class`))
  (if (> (`self.CurrentStraight`) 7)
    (`self.AddMapJump`)
    (else
      ;[1 1 1] 타일 불러오기
      (bind _returnvalue (`|SpawnActorFromClass` (`|GetArrayItem` _class (`KismetMathLibrary.RandomIntegerInRange` 0 (`KismetArrayLibrary.Array_LastIndex` _class))) (`self.NextSpawnPoint`) "Undefined" "OverrideRootScale" null null))
      (bind _asbp_master_tile (cast `/Game/Game/Tile/BP_MasterTile` _returnvalue))
      ;[1 1 1] 다음타일 위치
      (bind _attachpoint (`/Game/Game/Tile/BP_MasterTile.GetAttchTransform` _asbp_master_tile))
      ;[1 1 1] 다음 타일 위치 설정
      (set `self.NextSpawnPoint` _attachpoint)
      (set `self.CurrentStraight` (+ (`self.CurrentStraight`) 1)))))

(fn `AddMapJump`
  (bind _jump (`self.Jump`))
  ;[1 1 1] 타일 불러오기
  (bind _returnvalue (`|SpawnActorFromClass` (`|GetArrayItem` _jump (`KismetMathLibrary.RandomIntegerInRange` 0 (`KismetArrayLibrary.Array_LastIndex` _jump))) (`self.NextSpawnPoint`) "Undefined" "OverrideRootScale" null null))
  (bind _asbp_master_tile (cast `/Game/Game/Tile/BP_MasterTile` _returnvalue))
  ;[1 1 1] 다음타일 위치
  (bind _attachpoint (`/Game/Game/Tile/BP_MasterTile.GetAttchTransform` _asbp_master_tile))
  ;[1 1 1] 다음 타일 위치 설정
  (set `self.NextSpawnPoint` _attachpoint)
  (set `self.CurrentStraight` 0))

(fn `IncrementScore`
  ;[1 1 1] +1..+1..+1...
  (bind _result (`/Engine/EditorBlueprintResources/StandardMacros.IncrementInt` (`self.Score`))
    (:`  `
      (set `self.Score` _result))))

(fn `UserConstructionScript`)