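; Endless-runner track tile that populates itself on BeginPlay and exposes an attach point for chaining tiles.
; Child actor components place a random obstacle, lamps, coins in box areas, and an extra hard obstacle above a player speed threshold; pendulum and cannonball hazards spawn by chance.
; The end trigger asks BP_GameMode for another tile, raises player speed within limits, then destroys this one.
; Side walls apply hit-normal impulses; a box kills the player.
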(event `self.ReceiveBeginPlay`
  (`self.SetSpawnPoints`)
  (`self.SetObstacles`)
  (`self.SpawnObstacles`)
  (`self.SpawnObstaclesNew`)
  (`self.SpawnCoins`))

(event `self.EndTrigger.OnComponentBeginOverlap`
  (params (OverlappedComponent :type "PrimitiveComponent Object Reference") (OtherActor :type "Actor Object Reference") (OtherComp :type "PrimitiveComponent Object Reference") (OtherBodyIndex :type Integer) (bFromSweep :type Boolean) (SweepResult :type "HitResult Structure (by ref)"))
  ;[1 1 1] Add Map 불러와야 해서 필요함
  (bind _asbp_game_mode (cast `/Game/Game/GameMode/BP_GameMode` (`GameplayStatics.GetGameMode`)))
  (`/Game/Game/GameMode/BP_GameMode.AddMap` _asbp_game_mode)
  ;[1 1 1] 타일 지날때마다 스피드 올리기
  (bind _asmy_char (cast `/Game/Game/Character/My_Char` (`GameplayStatics.GetPlayerCharacter` 0)))
  (bind _charactermovement (`Character.CharacterMovement` _asmy_char))
  (set `CharacterMovementComponent.MaxWalkSpeed` (`KismetMathLibrary.FClamp` (* (`CharacterMovementComponent.MaxWalkSpeed` _charactermovement) 1.05) 600.0 1800.0) _charactermovement)
  (`KismetSystemLibrary.Delay` 2.0)
  (`self.K2_DestroyActor`))

(event `self.BounceWallL.OnComponentHit`
  (params (HitComponent :type "PrimitiveComponent Object Reference") (OtherActor :type "Actor Object Reference") (OtherComp :type "PrimitiveComponent Object Reference") (NormalImpulse :type "Vector Structure") (Hit :type "HitResult Structure (by ref)"))
  (bind _asmy_char (cast `/Game/Game/Character/My_Char` OtherActor))
  (`/Game/Game/Character/My_Char.ApplyImpulse` _asmy_char (* (`.Normal` (`GameplayStatics.BreakHitResult` Hit)) -7)))

(event `self.BounceWallR.OnComponentHit`
  (params (HitComponent :type "PrimitiveComponent Object Reference") (OtherActor :type "Actor Object Reference") (OtherComp :type "PrimitiveComponent Object Reference") (NormalImpulse :type "Vector Structure") (Hit :type "HitResult Structure (by ref)"))
  (bind _asmy_char (cast `/Game/Game/Character/My_Char` OtherActor))
  (`/Game/Game/Character/My_Char.ApplyImpulse` _asmy_char (* (`.Normal` (`GameplayStatics.BreakHitResult` Hit)) -7)))

(event `self.Box.OnComponentBeginOverlap`
  (params (OverlappedComponent :type "PrimitiveComponent Object Reference") (OtherActor :type "Actor Object Reference") (OtherComp :type "PrimitiveComponent Object Reference") (OtherBodyIndex :type Integer) (bFromSweep :type Boolean) (SweepResult :type "HitResult Structure (by ref)"))
  (bind _asmy_char (cast `/Game/Game/Character/My_Char` OtherActor))
  (`/Game/Game/Character/My_Char.Death` _asmy_char))

(fn `GetAttchTransform`
  (returns (AttachPoint :type "Transform Structure"))
  ;[1 1 1] Tile 이어지는 포인트
  (return (`SceneComponent.K2_GetComponentToWorld` (`self.AttachPoint`))))

(fn `SetObstacles`
  (`|ExecutionSequence`
    (:`then_0`
      (set `self.Obstacles` (`|MakeArray` "/Game/Game/Blueprint/BP_Obstacle4.BP_Obstacle4_C" "/Game/Game/Blueprint/BP_Obstacle3.BP_Obstacle3_C" "/Game/Game/Blueprint/BP_Obstacle4.BP_Obstacle4_C" "/Game/Game/Blueprint/BP_Truck.BP_Truck_C" :!type "Actor Class Reference")))
    (:`then_1`
      (set `self.ObstaclesHard` (`|MakeArray` "/Game/Game/Blueprint/BP_Airplane.BP_Airplane_C" "/Game/Game/Blueprint/BP_Airplane.BP_Airplane_C" "/Game/Game/Blueprint/BP_Airplane.BP_Airplane_C" :!type "Actor Class Reference")))
    (:`then_2`
      (set `self.ObstaclesHardLamp` "/Game/Game/Blueprint/BP_Lamp.BP_Lamp_C"))))

(fn `SetSpawnPoints`
  (`|ExecutionSequence`
    (:`then_0`
      (set `self.SpawnPoints` (`|MakeArray` (`SceneComponent.GetRelativeTransform` (`self.SpawnR`)) (`SceneComponent.GetRelativeTransform` (`self.SpawnL`)) (`SceneComponent.GetRelativeTransform` (`self.SpawnCenter`)))))
    (:`then_1`
      (set `self.SpawnPointsHard` (`|MakeArray` (`SceneComponent.GetRelativeTransform` (`self.LaneLeft`)) (`SceneComponent.GetRelativeTransform` (`self.LaneRight`)))))
    (:`then_2`
      (set `self.SpawnPointsLamp` (`|MakeArray` (`SceneComponent.GetRelativeTransform` (`self.LampL1`)) (`SceneComponent.GetRelativeTransform` (`self.LampR1`)))))))

(fn `SpawnCoins`
  (bind _coinarea (`self.CoinArea`))
  (bind _coinarea1 (`self.CoinArea1`))
  (`|ExecutionSequence`
    (:`then_0`
      (for _ (range 2)
        (`AddComponent|NODE_AddChildActorComponent-3` :`RelativeTransform` (`KismetMathLibrary.Conv_VectorToTransform` (`KismetMathLibrary.RandomPointInBoundingBox` (`SceneComponent.RelativeLocation` _coinarea) (`BoxComponent.BoxExtent` _coinarea))))))
    (:`then_1`
      (for _ (range 2)
        (`AddComponent|NODE_AddChildActorComponent-4` :`RelativeTransform` (`KismetMathLibrary.Conv_VectorToTransform` (`KismetMathLibrary.RandomPointInBoundingBox` (`SceneComponent.RelativeLocation` _coinarea1) (`BoxComponent.BoxExtent` _coinarea1))))))))

(fn `SpawnObstacles`
  (bind _spawnpoints (`self.SpawnPoints`))
  (bind _obstacles (`self.Obstacles`))
  (bind _spawnpointshard (`self.SpawnPointsHard`))
  (bind _obstacleshard (`self.ObstaclesHard`))
  (`|ExecutionSequence`
    (:`then_0`
      (bind _returnvalue (`AddComponent|NODE_AddChildActorComponent-0` :`RelativeTransform` (`|GetArrayItem` _spawnpoints (`KismetMathLibrary.RandomIntegerInRange` 0 (`KismetArrayLibrary.Array_LastIndex` _spawnpoints)))))
      (`ChildActorComponent.SetChildActorClass` _returnvalue (`|GetArrayItem` _obstacles (`KismetMathLibrary.RandomIntegerInRange` 0 (`KismetArrayLibrary.Array_LastIndex` _obstacles)))))
    (:`then_1`
      (bind _asmy_char (cast `/Game/Game/Character/My_Char` (`GameplayStatics.GetPlayerCharacter` 0)))
      (if (< 1000.0 (`MovementComponent.GetMaxSpeed` (`Character.CharacterMovement` _asmy_char)))
        (bind _returnvalue_2 (`AddComponent|NODE_AddChildActorComponent-1` :`RelativeTransform` (`|GetArrayItem` _spawnpointshard (`KismetMathLibrary.RandomIntegerInRange` 0 (`KismetArrayLibrary.Array_LastIndex` _spawnpointshard)))))
        (`ChildActorComponent.SetChildActorClass` _returnvalue_2 (`|GetArrayItem` _obstacleshard (`KismetMathLibrary.RandomIntegerInRange` 0 (`KismetArrayLibrary.Array_LastIndex` _obstacleshard))))))
    (:`then_2`
      (for _array_element (`self.SpawnPointsLamp`)
        (bind _returnvalue_3 (`AddComponent|NODE_AddChildActorComponent-2` :`RelativeTransform` _array_element))
        (`ChildActorComponent.SetChildActorClass` _returnvalue_3 "/Game/Game/Blueprint/BP_Lamp.BP_Lamp_C")))))

(fn `SpawnObstaclesNew`
  (`|ExecutionSequence`
    (:`then_0`
      ;[1 1 1] LaneL
      (switch `int` (`KismetMathLibrary.RandomIntegerInRange` 0 3)
        (:`1`
          (`|SpawnActorFromClass` "/Game/Game/Blueprint/BP_Obstacle5.BP_Obstacle5_C" (`SceneComponent.K2_GetComponentToWorld` (`self.Pendulum`)) "Undefined" "OverrideRootScale" null null))))
    (:`then_1`
      (switch `int` (`KismetMathLibrary.RandomIntegerInRange` 0 3)
        (:`1`
          (`|SpawnActorFromClass` "/Game/Game/Blueprint/BP_CannonBall.BP_CannonBall_C" (`SceneComponent.K2_GetComponentToWorld` (`self.CannonL`)) "Undefined" "OverrideRootScale" null null))))
    (:`then_2`
      (switch `int` (`KismetMathLibrary.RandomIntegerInRange` 0 3)
        (:`1`
          (`|SpawnActorFromClass` "/Game/Game/Blueprint/BP_CannonBall.BP_CannonBall_C" (`SceneComponent.K2_GetComponentToWorld` (`self.CannonR`)) "Undefined" "OverrideRootScale" null null))))))

(fn `UserConstructionScript`)