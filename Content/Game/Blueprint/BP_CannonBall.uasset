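; Cannon hazard that tracks the player pawn and periodically fires a physics cannonball that kills My_Char on hit.
; Tick eases the Arrow's rotation toward the player, and a looping timer calls DoShoot to reuse one ball: snap it to the Arrow, zero its velocity, apply a forward impulse.
; On hit, it calls Death, pushes the character mesh along the ball-to-cannon direction and spawns an emitter.
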(event `self.ReceiveBeginPlay`
  ;[1 1 1] 목표 구하기
  (set `self.Target` (`GameplayStatics.GetPlayerPawn` 0))
  (`self.DoShoot`)
  ;[1 1 1] 2초 마다 쏜다
  (`KismetSystemLibrary.K2_SetTimer` null "DoShoot" 3.0 true)
  (`GameplayStatics.PlaySound2D` "/Game/Game/Sound/SFX_Ball.SFX_Ball" 0.5 1.0 0.0 null null false))

(event `self.ReceiveTick`
  (params (DeltaSeconds :type "Float (single-precision)"))
  (bind _arrow (`self.Arrow`))
  ;[1 1 1] Cannon 머리 돌아가기
  (`SceneComponent.K2_SetWorldRotation` _arrow (`KismetMathLibrary.RLerp` (`SceneComponent.K2_GetComponentRotation` _arrow) (`KismetMathLibrary.FindLookAtRotation` (`SceneComponent.K2_GetComponentLocation` _arrow) (`self.K2_GetActorLocation` (`self.Target`))) 0.05 true) false false))

(event `self.CannonBall.OnComponentHit`
  (params (HitComponent :type "PrimitiveComponent Object Reference") (OtherActor :type "Actor Object Reference") (OtherComp :type "PrimitiveComponent Object Reference") (NormalImpulse :type "Vector Structure") (Hit :type "HitResult Structure (by ref)"))
  (bind _returnvalue (`SceneComponent.K2_GetComponentLocation` (`self.CannonBall`)))
  (bind _asmy_char (cast `/Game/Game/Character/My_Char` OtherActor))
  (`/Game/Game/Character/My_Char.Death` _asmy_char)
  (`PrimitiveComponent.AddImpulse` (`Character.Mesh` _asmy_char) (* (`KismetMathLibrary.GetForwardVector` (`KismetMathLibrary.FindLookAtRotation` _returnvalue (`self.K2_GetActorLocation`))) 100000.0) "None" false)
  (`GameplayStatics.SpawnEmitterAtLocation` null _returnvalue))

(fn `DoShoot`
  (bind _cannonball (`self.CannonBall`))
  (bind _arrow (`self.Arrow`))
  ;[1 1 1] 위치값을 설정한다
  (`SceneComponent.K2_SetWorldLocationAndRotation` (`self.CannonBall`) (`SceneComponent.K2_GetComponentLocation` _arrow) (`SceneComponent.K2_GetComponentRotation` _arrow) false false)
  ;[1 1 1] 캐논 쏘는것
  ;;[1 1 1] Cannon  초기화 해준다
  (`PrimitiveComponent.SetAllPhysicsLinearVelocity` _cannonball (0.0 0.0 0.0) false)
  ;;[1 1 1] 단발성 물리력을 줬지만, 발사후에 Impulse 각도가 달라진다.
  (`PrimitiveComponent.AddImpulse` _cannonball (* (`SceneComponent.GetForwardVector` _cannonball) 200000.0) "None" false))

(fn `UserConstructionScript`)