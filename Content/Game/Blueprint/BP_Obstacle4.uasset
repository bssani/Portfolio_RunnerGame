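; BP_Obstacle4 is a moving hazard that slides sideways and kills any My_Char that overlaps its Cube.
; On the authority, a timeline with play rate set from RepeatTime offsets the root along the actor's right vector, scaled by Distance, without sweeping.
; Actor overlaps with locally controlled players toggle FixShake, a movement fix for stationary players hit by the obstacle.
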(event `self.ReceiveBeginPlay`
  (`/Engine/EditorBlueprintResources/ActorMacros.Switch Has Authority`
    (:`Authority`
      (bind _output_get (set `self.RootLocation` (`SceneComponent.K2_GetComponentLocation` (`self.DefaultSceneRoot`))))
      (`TimelineComponent.SetPlayRate` (`self.Timeline_0`) (/ 1.0 (`self.RepeatTime`)))
      (bind (_direction _newtrack_2) (`Timeline|Timeline_0`)
        (:`Update`
          (`SceneComponent.K2_SetWorldLocation` (`self.DefaultSceneRoot`) (+ (* (`self.GetActorRightVector`) (* (* _newtrack_2 (`self.Distance`)) 100.0)) _output_get) false false))))))

(event `self.ReceiveActorBeginOverlap`
  (params (OtherActor :type "Actor Object Reference"))
  ;[1 1 1] Player movement fix when is stopped and hits with this actor
  (if (`self.ActorHasTag` OtherActor "Player")
    (bind _asmy_char (cast `/Game/Game/Character/My_Char` OtherActor))
    (if (`Pawn.IsLocallyControlled` _asmy_char)
      (`/Game/Game/Character/My_Char.FixShake` _asmy_char true))))

(event `self.ReceiveActorEndOverlap`
  (params (OtherActor :type "Actor Object Reference"))
  ;[1 1 1] Player movement fix when is stopped and hits with this actor
  (if (`self.ActorHasTag` OtherActor "Player")
    (bind _asmy_char (cast `/Game/Game/Character/My_Char` OtherActor))
    (if (`Pawn.IsLocallyControlled` _asmy_char)
      (`/Game/Game/Character/My_Char.FixShake` _asmy_char false))))

(event `self.Cube.OnComponentBeginOverlap`
  (params (OverlappedComponent :type "PrimitiveComponent Object Reference") (OtherActor :type "Actor Object Reference") (OtherComp :type "PrimitiveComponent Object Reference") (OtherBodyIndex :type Integer) (bFromSweep :type Boolean) (SweepResult :type "HitResult Structure (by ref)"))
  (bind _asmy_char (cast `/Game/Game/Character/My_Char` OtherActor))
  (`/Game/Game/Character/My_Char.Death` _asmy_char))

(fn `UserConstructionScript`)