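; BP_Obstacle3 is a deadly moving obstacle that calls Death on any My_Char registering a hit on its Cube.
; On BeginPlay, only the authority stores the root's start location and plays a timeline with its rate set by RepeatTime.
; The timeline track, scaled by Distance, offsets the root along the actor's negative up axis from that start, without sweeping.
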(event `self.ReceiveBeginPlay`
  (`/Engine/EditorBlueprintResources/ActorMacros.Switch Has Authority`
    (:`Authority`
      (bind _output_get (set `self.RootLocation` (`SceneComponent.K2_GetComponentLocation` (`self.DefaultSceneRoot`))))
      (`TimelineComponent.SetPlayRate` (`self.Timeline_0`) (/ 1.0 (`self.RepeatTime`)))
      (bind (_direction _newtrack_2) (`Timeline|Timeline_0`)
        (:`Update`
          (`SceneComponent.K2_SetWorldLocation` (`self.DefaultSceneRoot`) (+ (* (`self.GetActorUpVector`) (* (* _newtrack_2 (`self.Distance`)) -100.0)) _output_get) false false))))))

(event `self.Cube.OnComponentHit`
  (params (HitComponent :type "PrimitiveComponent Object Reference") (OtherActor :type "Actor Object Reference") (OtherComp :type "PrimitiveComponent Object Reference") (NormalImpulse :type "Vector Structure") (Hit :type "HitResult Structure (by ref)"))
  (bind _asmy_char (cast `/Game/Game/Character/My_Char` OtherActor))
  (`/Game/Game/Character/My_Char.Death` _asmy_char))

(fn `UserConstructionScript`)