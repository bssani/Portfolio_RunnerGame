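; BP_Obstacle5 is a swinging obstacle that knocks back and kills any My_Char that hits its Sphere.
; On the server, Tick pins the actor at Origin and oscillates its pitch with a sine of game time, scaled by Speed and MaxAngle.
; A Sphere hit applies an impulse against the hit normal, then calls Death on the character.
; The Player-tag overlap handlers, meant as a movement fix, currently do nothing.
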(event `self.ReceiveTick`
  (params (DeltaSeconds :type "Float (single-precision)"))
  (`/Engine/EditorBlueprintResources/ActorMacros.Switch Has Authority`
    (:`Authority`
      (`self.K2_SetActorLocationAndRotation` (`SceneComponent.K2_GetComponentLocation` (`self.Origin`)) (`KismetMathLibrary.MakeRotator` 0.0 (* (`KismetMathLibrary.Sin` (* (`self.Speed`) (`GameplayStatics.GetTimeSeconds`))) (`self.MaxAngle`)))))))

(event `self.Sphere.OnComponentHit`
  (params (HitComponent :type "PrimitiveComponent Object Reference") (OtherActor :type "Actor Object Reference") (OtherComp :type "PrimitiveComponent Object Reference") (NormalImpulse :type "Vector Structure") (Hit :type "HitResult Structure (by ref)"))
  ;[1 1 1] Apply a force opposite to the direction of hit to the player
  (bind _asmy_char (cast `/Game/Game/Character/My_Char` OtherActor))
  (`/Game/Game/Character/My_Char.ApplyImpulse` _asmy_char (* (`.Normal` (`GameplayStatics.BreakHitResult` Hit)) -3))
  (`/Game/Game/Character/My_Char.Death` _asmy_char))

(event `self.ReceiveActorBeginOverlap`
  (params (OtherActor :type "Actor Object Reference"))
  ;[1 1 1] Player movement fix when is stopped and hits with this actor
  (if (`self.ActorHasTag` OtherActor "Player")
    _))

(event `self.ReceiveActorEndOverlap`
  (params (OtherActor :type "Actor Object Reference"))
  ;[1 1 1] Player movement fix when is stopped and hits with this actor
  (if (`self.ActorHasTag` OtherActor "Player")
    _))

(fn `UserConstructionScript`)